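; Attack particle actor for virtual pet training that reacts to hitting a training punching bag.
; A delayed flip-flop on Tick alternates two Paper2D sprites for a simple animation.
; Overlapping the bag plays a sound, resets the first VPet's training event, restarts it while HitCount is below four, then destroys the particle.
; FaceCamera yaws the sprite toward the player's camera but is not called within this Blueprint.
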(event `self.ReceiveBeginPlay`
  (bind _asfirst_person_character (cast `/Game/FirstPersonBP/Blueprints/FirstPersonCharacter` (`GameplayStatics.GetPlayerCharacter` 0)))
  (set `self.PlayerReference` _asfirst_person_character))

(event `self.ReceiveTick`
  (params (DeltaSeconds :type "Float (single-precision)"))
  (bind _papersprite (`self.PaperSprite`))
  (`KismetSystemLibrary.Delay` 0.5)
  (`/Engine/EditorBlueprintResources/StandardMacros.FlipFlop`
    (:`A`
      (`PaperSpriteComponent.SetSprite` _papersprite (`self.AttackParticle1`)))
    (:`B`
      (`PaperSpriteComponent.SetSprite` _papersprite (`self.AttackParticle2`)))))

(event `self.Sphere.OnComponentBeginOverlap`
  (params (OverlappedComponent :type "PrimitiveComponent Object Reference") (OtherActor :type "Actor Object Reference") (OtherComp :type "PrimitiveComponent Object Reference") (OtherBodyIndex :type Integer) (bFromSweep :type Boolean) (SweepResult :type "HitResult Structure (by ref)"))
  (bind _astraining_punching_bag_bp (cast `/Game/Main/BP/TrainingPunchingBag_BP` OtherActor))
  (`/Engine/EditorBlueprintResources/StandardMacros.IsValid` self
    (:`Is Valid`
      (`GameplayStatics.PlaySound2D` "/Game/Retro_8Bit_Sounds/Retro_Orginal/Cues/retro_synth_beeps_groove_06_Cue.retro_synth_beeps_groove_06_Cue" 1.0 1.0 0.0 null null)
      (bind _outactors (`GameplayStatics.GetAllActorsOfClass` "/Game/Main/BP/VPet_BP.VPet_BP_C"))
      (bind _output (`|GetArrayItem` _outactors))
      (`/Game/Main/BP/VPet_BP.ResetTrainingEvent` _output)
      (if (< (`/Game/Main/BP/TrainingPunchingBag_BP.HitCount` _astraining_punching_bag_bp) 4)
        (`/Game/Main/BP/VPet_BP.TrainingEvent` _output)
        (else
          (`/Game/Main/BP/VPet_BP.ResetTrainingEvent` _output)))
      (`self.K2_DestroyActor`))))

(fn `FaceCamera`
  (bind _papersprite (`self.PaperSprite`))
  (bind (_returnvalue_roll _returnvalue_pitch _returnvalue_yaw) (`KismetMathLibrary.BreakRotator` (`KismetMathLibrary.FindLookAtRotation` (`SceneComponent.K2_GetComponentLocation` _papersprite) (`SceneComponent.K2_GetComponentLocation` (`/Game/FirstPersonBP/Blueprints/FirstPersonCharacter.FirstPersonCamera` (`self.PlayerReference`))))))
  (`SceneComponent.K2_SetWorldRotation` _papersprite (`KismetMathLibrary.MakeRotator` 0.0 0.0 (- _returnvalue_yaw 90.0)) false false))

(fn `UserConstructionScript`)