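; Punching bag actor for virtual pet training, hidden until StartTraining runs.
; StartTraining, gated by a DoOnce that ResetCanTrainNeomon re-arms, moves the pet to the training position and starts its training unless eating, an egg or battling.
; Attack particle overlaps flash a hit sprite and count hits.
; The fifth hit plays a sound and destroyed sprite, then after a delay ends pet training and hides the bag.
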(event `self.ReceiveBeginPlay`
  (`self.SetActorHiddenInGame` true))

(event `self.Capsule.OnComponentBeginOverlap`
  (params (OverlappedComponent :type "PrimitiveComponent Object Reference") (OtherActor :type "Actor Object Reference") (OtherComp :type "PrimitiveComponent Object Reference") (OtherBodyIndex :type Integer) (bFromSweep :type Boolean) (SweepResult :type "HitResult Structure (by ref)"))
  (cast `/Game/Main/BP/VPETAttackParticle_BP` OtherActor)
  (`PaperSpriteComponent.SetSprite` (`self.PaperSprite`) "/Game/Main/UI/Asset/PunchingBagHit_T_Sprite.PunchingBagHit_T_Sprite")
  (bind _output_get (set `self.HitCount` (+ (`self.HitCount`) 1)))
  (if (> _output_get 4)
    (`GameplayStatics.PlaySound2D` "/Game/Retro_8Bit_Sounds/Retro_Orginal/Cues/retro_synth_beeps_01_Cue.retro_synth_beeps_01_Cue" 1.0 1.0 0.0 null null)
    (`PaperSpriteComponent.SetSprite` (`self.PaperSprite`) "/Game/Main/UI/Asset/PunchingBagDestroyed_T_Sprite.PunchingBagDestroyed_T_Sprite")
    (`KismetSystemLibrary.Delay` 1.0)
    (bind _outactors (`GameplayStatics.GetAllActorsOfClass` "/Game/Main/BP/VPet_BP.VPet_BP_C"))
    (bind _output (`|GetArrayItem` _outactors))
    (set `/Game/Main/BP/VPet_BP.IsTraining` false _output)
    (`/Game/Main/BP/VPet_BP.SetVpetWalk` _output)
    (`/Game/Main/BP/VPet_BP.ResetTrainingEvent` _output)
    (set `self.HitCount` 0)
    (`self.SetActorHiddenInGame` true)
    (`PaperSpriteComponent.SetSprite` (`self.PaperSprite`) "/Game/Main/UI/Asset/PunchingBagIdle_T_Sprite.PunchingBagIdle_T_Sprite")
    (else
      (`KismetSystemLibrary.Delay` 1.0)
      (`PaperSpriteComponent.SetSprite` (`self.PaperSprite`) "/Game/Main/UI/Asset/PunchingBagIdle_T_Sprite.PunchingBagIdle_T_Sprite"))))

(event `StartTraining`
  (`/Engine/EditorBlueprintResources/StandardMacros.DoOnce` false :!label _label
    (:`Completed`
      (bind _outactors (`GameplayStatics.GetAllActorsOfClass` "/Game/Main/BP/VPet_BP.VPet_BP_C"))
      (bind _output (`|GetArrayItem` _outactors))
      (if (`/Game/Main/BP/VPet_BP.IsEating` _output)
        _
        (elif (`/Game/Main/BP/VPet_BP.IsEgg` _output)
          _
          (elif (not (`/Game/Main/BP/VPet_BP.IsInBattle` _output))
            (`self.SetActorHiddenInGame` false)
            (bind _outactors_2 (`GameplayStatics.GetAllActorsOfClass` "/Game/Main/BP/VPETAttackTrainingPos.VPETAttackTrainingPos_C"))
            (`self.K2_SetActorLocation` _output (`self.K2_GetActorLocation` (`|GetArrayItem` _outactors_2)) false false)
            (if (not (`/Game/Main/BP/VPet_BP.IsTraining` _output))
              (set `/Game/Main/BP/VPet_BP.IsTraining` true _output)
              (`/Game/Main/BP/VPet_BP.TrainingEvent` _output))))))))

(event `ResetCanTrainNeomon`
  (goto _label :!via `Reset`))

(fn `UserConstructionScript`)