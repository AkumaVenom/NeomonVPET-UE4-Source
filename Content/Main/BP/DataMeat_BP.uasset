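; DataMeat is a short-lived food actor that plays out an eating sequence for the virtual pet and restores player hunger.
; On BeginPlay it steps through shrinking meat sprites with timed retro beeps, then adds clamped hunger to the FirstPersonCharacter.
; It finally clears IsEating on the first VPet_BP, calls ResetCanEat on the player and destroys itself.
; A FacePlayer function yaw-billboards the sprite toward the camera but is not called here.
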(event `self.ReceiveBeginPlay`
  (bind _playerreference (`self.PlayerReference`))
  (bind _maxhunger (`/Game/FirstPersonBP/Blueprints/FirstPersonCharacter.MaxHunger` _playerreference))
  (bind _asfirst_person_character (cast `/Game/FirstPersonBP/Blueprints/FirstPersonCharacter` (`GameplayStatics.GetPlayerCharacter` 0)))
  (set `self.PlayerReference` _asfirst_person_character)
  (`GameplayStatics.PlaySound2D` "/Game/Retro_8Bit_Sounds/Retro_Orginal/Cues/retro_beeps_success_04_Cue.retro_beeps_success_04_Cue" 1.0 1.0 0.0 null null)
  (`KismetSystemLibrary.Delay` 1.0)
  (`GameplayStatics.PlaySound2D` "/Game/Retro_8Bit_Sounds/Retro_Orginal/Cues/retro_beeps_success_04_Cue.retro_beeps_success_04_Cue" 1.0 1.0 0.0 null null)
  (`PaperSpriteComponent.SetSprite` (`self.PaperSprite`) "/Game/Main/UI/Asset/DataMeatMiddle_T_Sprite.DataMeatMiddle_T_Sprite")
  (`KismetSystemLibrary.Delay` 1.0)
  (`GameplayStatics.PlaySound2D` "/Game/Retro_8Bit_Sounds/Retro_Orginal/Cues/retro_beeps_success_04_Cue.retro_beeps_success_04_Cue" 1.0 1.0 0.0 null null)
  (`PaperSpriteComponent.SetSprite` (`self.PaperSprite`) "/Game/Main/UI/Asset/DataMeatLast_T_Sprite.DataMeatLast_T_Sprite")
  (`KismetSystemLibrary.Delay` 1.0)
  (`GameplayStatics.PlaySound2D` "/Game/Retro_8Bit_Sounds/Retro_Orginal/Cues/retro_beeps_success_04_Cue.retro_beeps_success_04_Cue" 1.0 1.0 0.0 null null)
  (bind _output_get (set `/Game/FirstPersonBP/Blueprints/FirstPersonCharacter.CurrentHunger` (+ (`/Game/FirstPersonBP/Blueprints/FirstPersonCharacter.CurrentHunger` _playerreference) 40) _playerreference))
  (if (> _output_get _maxhunger)
    (set `/Game/FirstPersonBP/Blueprints/FirstPersonCharacter.CurrentHunger` _maxhunger _playerreference))
  (bind _outactors (`GameplayStatics.GetAllActorsOfClass` "/Game/Main/BP/VPet_BP.VPet_BP_C"))
  (set `/Game/Main/BP/VPet_BP.IsEating` false (`|GetArrayItem` _outactors))
  (`/Game/FirstPersonBP/Blueprints/FirstPersonCharacter.ResetCanEat` (`self.PlayerReference`))
  (`/Engine/EditorBlueprintResources/StandardMacros.IsValid` self
    (:`Is Valid`
      (`self.K2_DestroyActor`))))

(fn `FacePlayer`
  (bind _papersprite (`self.PaperSprite`))
  (bind (_returnvalue_roll _returnvalue_pitch _returnvalue_yaw) (`KismetMathLibrary.BreakRotator` (`KismetMathLibrary.FindLookAtRotation` (`SceneComponent.K2_GetComponentLocation` _papersprite) (`SceneComponent.K2_GetComponentLocation` (`/Game/FirstPersonBP/Blueprints/FirstPersonCharacter.FirstPersonCamera` (`self.PlayerReference`))))))
  (`SceneComponent.K2_SetWorldRotation` _papersprite (`KismetMathLibrary.MakeRotator` 0.0 0.0 (- _returnvalue_yaw 90.0)) false false))

(fn `UserConstructionScript`)