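; Virtual pet character drawn as billboarded 2D sprites that face the player camera, starting as an egg or one of five baby slimes.
; The egg sounds an alarm, picks a random slime, updates the player's flags and destroys itself.
; Slimes load sprites from those flags, roam between marker actors, eat, poop with cleaning alerts, and attack a training bag.
; A dot product against the player selects left or right walk/idle frames.
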(event `self.ReceiveBeginPlay`
  (bind _asfirst_person_character (cast `/Game/FirstPersonBP/Blueprints/FirstPersonCharacter` (`GameplayStatics.GetPlayerCharacter` 0)))
  (set `self.PlayerReference` _asfirst_person_character)
  (`KismetSystemLibrary.Delay` 1.0)
  (bind _playerreference (`self.PlayerReference`)
    (:`then`
      (set `self.NeedsCleaning` (`/Game/FirstPersonBP/Blueprints/FirstPersonCharacter.NeedCleaning` _playerreference))
      (if (`self.IsEgg`)
        (set `self.Idle1_Left` "/Game/Main/UI/Asset/RedStipeEgg1_T_Sprite.RedStipeEgg1_T_Sprite")
        (set `self.Idle2_Left` "/Game/Main/UI/Asset/RedStipeEgg2_T_Sprite.RedStipeEgg2_T_Sprite")
        (elif (`/Game/FirstPersonBP/Blueprints/FirstPersonCharacter.IsBabySlime1` (`self.PlayerReference`))
          (set `self.Idle1_Left` "/Game/Main/VPET/2DNeomon/Nano/BabySlime1/BabySlime1_Idle1_Sprite.BabySlime1_Idle1_Sprite" :!label _label)
          (set `self.Idle2_Left` "/Game/Main/VPET/2DNeomon/Nano/BabySlime1/BabySlime1_Idle2_Sprite.BabySlime1_Idle2_Sprite")
          (set `self.LLegWalkLeft` "/Game/Main/VPET/2DNeomon/Nano/BabySlime1/BabySlime1_LLegWalk_Sprite.BabySlime1_LLegWalk_Sprite")
          (set `self.RLegWalkLeft` "/Game/Main/VPET/2DNeomon/Nano/BabySlime1/BabySlime1_RLegWalk_Sprite.BabySlime1_RLegWalk_Sprite")
          (set `self.Attack` "/Game/Main/VPET/2DNeomon/Nano/BabySlime1/BabySlime1_Attack_Sprite.BabySlime1_Attack_Sprite")
          (set `self.Eat` "/Game/Main/VPET/2DNeomon/Nano/BabySlime1/BabySlime1_Eat_Sprite.BabySlime1_Eat_Sprite")
          (set `self.GetHit` "/Game/Main/VPET/2DNeomon/Nano/BabySlime1/BabySlime1_GetHit_Sprite.BabySlime1_GetHit_Sprite")
          (set `self.AttackParticleClass` "/Game/Main/BP/VPETAttackParticle__BabySlime_LightPurple.VPETAttackParticle__BabySlime_LightPurple_C")
          (set `self.Idle1_Right` "/Game/Main/VPET/2DNeomon/Nano/BabySlime1/BabySlime1_Idle1_Right_Sprite.BabySlime1_Idle1_Right_Sprite")
          (set `self.Idle2_Right` "/Game/Main/VPET/2DNeomon/Nano/BabySlime1/BabySlime1_Idle2_Right_Sprite.BabySlime1_Idle2_Right_Sprite")
          (set `self.LLegWalk_Right` "/Game/Main/VPET/2DNeomon/Nano/BabySlime1/BabySlime1_LLegWalk_Right_Sprite.BabySlime1_LLegWalk_Right_Sprite")
          (set `self.RLegWalk_Right` "/Game/Main/VPET/2DNeomon/Nano/BabySlime1/BabySlime1_RLegWalk_Right_Sprite.BabySlime1_RLegWalk_Right_Sprite")
          (`SceneComponent.SetWorldScale3D` (`self.NPC`) (0.5 0.5 0.5))
          (elif (`/Game/FirstPersonBP/Blueprints/FirstPersonCharacter.IsBabySlime2` (`self.PlayerReference`))
            (set `self.Idle1_Left` "/Game/Main/VPET/2DNeomon/Nano/BabySlime2/BabySlime2_Idle1_Left_Sprite.BabySlime2_Idle1_Left_Sprite" :!label _label_2)
            (set `self.Idle2_Left` "/Game/Main/VPET/2DNeomon/Nano/BabySlime2/BabySlime2_Idle2_Left_Sprite.BabySlime2_Idle2_Left_Sprite")
            (set `self.LLegWalkLeft` "/Game/Main/VPET/2DNeomon/Nano/BabySlime2/BabySlime2_LLegWalk_Left_Sprite.BabySlime2_LLegWalk_Left_Sprite")
            (set `self.RLegWalkLeft` "/Game/Main/VPET/2DNeomon/Nano/BabySlime2/BabySlime2_RLegWalk_Left_Sprite.BabySlime2_RLegWalk_Left_Sprite")
            (set `self.Attack` "/Game/Main/VPET/2DNeomon/Nano/BabySlime2/BabySlime2_Attack_Left_Sprite.BabySlime2_Attack_Left_Sprite")
            (set `self.Eat` "/Game/Main/VPET/2DNeomon/Nano/BabySlime2/BabySlime2_Attack_Left_Sprite.BabySlime2_Attack_Left_Sprite")
            (set `self.GetHit` "/Game/Main/VPET/2DNeomon/Nano/BabySlime2/BabySlime2_GetHit_Left_Sprite.BabySlime2_GetHit_Left_Sprite")
            (set `self.AttackParticleClass` "/Game/Main/BP/VPETAttackParticle__BabySlime_Yellow.VPETAttackParticle__BabySlime_Yellow_C")
            (set `self.Idle1_Right` "/Game/Main/VPET/2DNeomon/Nano/BabySlime2/BabySlime2_Idle1_Right_Sprite.BabySlime2_Idle1_Right_Sprite")
            (set `self.Idle2_Right` "/Game/Main/VPET/2DNeomon/Nano/BabySlime2/BabySlime2_Idle2_Right_Sprite.BabySlime2_Idle2_Right_Sprite")
            (set `self.LLegWalk_Right` "/Game/Main/VPET/2DNeomon/Nano/BabySlime2/BabySlime2_LLegWalk_Right_Sprite.BabySlime2_LLegWalk_Right_Sprite")
            (set `self.RLegWalk_Right` "/Game/Main/VPET/2DNeomon/Nano/BabySlime2/BabySlime2_RLegWalk_Right_Sprite.BabySlime2_RLegWalk_Right_Sprite")
            (`SceneComponent.SetWorldScale3D` (`self.NPC`) (0.5 0.5 0.5))
            (elif (`/Game/FirstPersonBP/Blueprints/FirstPersonCharacter.IsBabySlime3` (`self.PlayerReference`))
              (set `self.Idle1_Left` "/Game/Main/VPET/2DNeomon/Nano/BabySlime3/BabySlime3_Idle1_Left_Sprite.BabySlime3_Idle1_Left_Sprite" :!label _label_3)
              (set `self.Idle2_Left` "/Game/Main/VPET/2DNeomon/Nano/BabySlime3/BabySlime3_Idle2_Left_Sprite.BabySlime3_Idle2_Left_Sprite")
              (set `self.LLegWalkLeft` "/Game/Main/VPET/2DNeomon/Nano/BabySlime3/BabySlime3_LLegWalk_Left_Sprite.BabySlime3_LLegWalk_Left_Sprite")
              (set `self.RLegWalkLeft` "/Game/Main/VPET/2DNeomon/Nano/BabySlime3/BabySlime3_RLeg_Left_Sprite.BabySlime3_RLeg_Left_Sprite")
              (set `self.Attack` "/Game/Main/VPET/2DNeomon/Nano/BabySlime3/BabySlime3_Attack_Left_Sprite.BabySlime3_Attack_Left_Sprite")
              (set `self.Eat` "/Game/Main/VPET/2DNeomon/Nano/BabySlime3/BabySlime3_Eat_Left_Sprite.BabySlime3_Eat_Left_Sprite")
              (set `self.GetHit` "/Game/Main/VPET/2DNeomon/Nano/BabySlime3/BabySlime3_GetHit_Left_Sprite.BabySlime3_GetHit_Left_Sprite")
              (set `self.AttackParticleClass` "/Game/Main/BP/VPETAttackParticle__BabySlime_Red.VPETAttackParticle__BabySlime_Red_C")
              (set `self.Idle1_Right` "/Game/Main/VPET/2DNeomon/Nano/BabySlime3/BabySlime3_Idle1_Right_Sprite.BabySlime3_Idle1_Right_Sprite")
              (set `self.Idle2_Right` "/Game/Main/VPET/2DNeomon/Nano/BabySlime3/BabySlime3_Idle2_Right_Sprite.BabySlime3_Idle2_Right_Sprite")
              (set `self.LLegWalk_Right` "/Game/Main/VPET/2DNeomon/Nano/BabySlime3/BabySlime3_LLegWalk_Right_Sprite.BabySlime3_LLegWalk_Right_Sprite")
              (set `self.RLegWalk_Right` "/Game/Main/VPET/2DNeomon/Nano/BabySlime3/BabySlime3_RLeg_Right_Sprite.BabySlime3_RLeg_Right_Sprite")
              (`SceneComponent.SetWorldScale3D` (`self.NPC`) (0.5 0.5 0.5))
              (elif (`/Game/FirstPersonBP/Blueprints/FirstPersonCharacter.IsBabySlime4` (`self.PlayerReference`))
                (set `self.Idle1_Left` "/Game/Main/VPET/2DNeomon/Nano/BabySlime4/BabySlime4_Idle1_Left_Sprite.BabySlime4_Idle1_Left_Sprite" :!label _label_4)
                (set `self.Idle2_Left` "/Game/Main/VPET/2DNeomon/Nano/BabySlime4/BabySlime4_Idle2_Left_Sprite.BabySlime4_Idle2_Left_Sprite")
                (set `self.LLegWalkLeft` "/Game/Main/VPET/2DNeomon/Nano/BabySlime4/BabySlime4_LLegWalk_Left_Sprite.BabySlime4_LLegWalk_Left_Sprite")
                (set `self.RLegWalkLeft` "/Game/Main/VPET/2DNeomon/Nano/BabySlime4/BabySlime4_RLegWalk_Left_Sprite.BabySlime4_RLegWalk_Left_Sprite")
                (set `self.Attack` "/Game/Main/VPET/2DNeomon/Nano/BabySlime4/BabySlime4_Attack_Left_Sprite.BabySlime4_Attack_Left_Sprite")
                (set `self.Eat` "/Game/Main/VPET/2DNeomon/Nano/BabySlime4/BabySlime4_Eat_Left_Sprite.BabySlime4_Eat_Left_Sprite")
                (set `self.GetHit` "/Game/Main/VPET/2DNeomon/Nano/BabySlime4/BabySlime4_GetHit_Left_Sprite.BabySlime4_GetHit_Left_Sprite")
                (set `self.AttackParticleClass` "/Game/Main/BP/VPETAttackParticle__BabySlime_LightBlue.VPETAttackParticle__BabySlime_LightBlue_C")
                (set `self.Idle1_Right` "/Game/Main/VPET/2DNeomon/Nano/BabySlime4/BabySlime4_Idle1_Right_Sprite.BabySlime4_Idle1_Right_Sprite")
                (set `self.Idle2_Right` "/Game/Main/VPET/2DNeomon/Nano/BabySlime4/BabySlime4_Idle2_Right_Sprite.BabySlime4_Idle2_Right_Sprite")
                (set `self.LLegWalk_Right` "/Game/Main/VPET/2DNeomon/Nano/BabySlime4/BabySlime4_LLegWalk_Right_Sprite.BabySlime4_LLegWalk_Right_Sprite")
                (set `self.RLegWalk_Right` "/Game/Main/VPET/2DNeomon/Nano/BabySlime4/BabySlime4_RLegWalk_Right_Sprite.BabySlime4_RLegWalk_Right_Sprite")
                (`SceneComponent.SetWorldScale3D` (`self.NPC`) (0.5 0.5 0.5))
                (elif (`/Game/FirstPersonBP/Blueprints/FirstPersonCharacter.IsBabySlime5` (`self.PlayerReference`))
                  (set `self.Idle1_Left` "/Game/Main/VPET/2DNeomon/Nano/BabySlime5/BabySlime5_Idle1_Left_Sprite.BabySlime5_Idle1_Left_Sprite" :!label _label_5)
                  (set `self.Idle2_Left` "/Game/Main/VPET/2DNeomon/Nano/BabySlime5/BabySlime5_Idle2_Left_Sprite.BabySlime5_Idle2_Left_Sprite")
                  (set `self.LLegWalkLeft` "/Game/Main/VPET/2DNeomon/Nano/BabySlime5/BabySlime5_LLegWalk_Left_Sprite.BabySlime5_LLegWalk_Left_Sprite")
                  (set `self.RLegWalkLeft` "/Game/Main/VPET/2DNeomon/Nano/BabySlime5/BabySlime5_RLegWalk_Left_Sprite.BabySlime5_RLegWalk_Left_Sprite")
                  (set `self.Attack` "/Game/Main/VPET/2DNeomon/Nano/BabySlime5/BabySlime5_Attack_Left_Sprite.BabySlime5_Attack_Left_Sprite")
                  (set `self.Eat` "/Game/Main/VPET/2DNeomon/Nano/BabySlime5/BabySlime5_LLegWalk_Left_Sprite.BabySlime5_LLegWalk_Left_Sprite")
                  (set `self.GetHit` "/Game/Main/VPET/2DNeomon/Nano/BabySlime5/BabySlime5_GetHit_Left_Sprite.BabySlime5_GetHit_Left_Sprite")
                  (set `self.AttackParticleClass` "/Game/Main/BP/VPETAttackParticle__BabySlime_LightGreen.VPETAttackParticle__BabySlime_LightGreen_C")
                  (set `self.Idle1_Right` "/Game/Main/VPET/2DNeomon/Nano/BabySlime5/BabySlime5_Idle1_Right_Sprite.BabySlime5_Idle1_Right_Sprite")
                  (set `self.Idle2_Right` "/Game/Main/VPET/2DNeomon/Nano/BabySlime5/BabySlime5_Idle2_Right_Sprite.BabySlime5_Idle2_Right_Sprite")
                  (set `self.LLegWalk_Right` "/Game/Main/VPET/2DNeomon/Nano/BabySlime5/BabySlime5_LLegWalk_Right_Sprite.BabySlime5_LLegWalk_Right_Sprite")
                  (set `self.RLegWalk_Right` "/Game/Main/VPET/2DNeomon/Nano/BabySlime5/BabySlime5_RLegWalk_Right_Sprite.BabySlime5_RLegWalk_Right_Sprite")
                  (`SceneComponent.SetWorldScale3D` (`self.NPC`) (0.5 0.5 0.5)))))))))
    (:`else`)))

(event `SetBabySlime1`
  (goto _label))

(event `SetBabySlime2`
  (goto _label_2))

(event `SetBabySlime3`
  (goto _label_3))

(event `SetBabySlime4`
  (goto _label_4))

(event `SetBabySlime5`
  (goto _label_5))

(event `self.ReceiveTick`
  (params (DeltaSeconds :type "Float (single-precision)"))
  (`self.FacePlayerCamera`)
  (if (`self.IsTraining`)
    (`self.TrainingEvent`)
    (elif (`self.IsEgg`)
      ;[1 1 1] EGG LOGIC
      (`|ExecutionSequence`
        (:`then_0`
          (`KismetSystemLibrary.Delay` 0.7)
          (if (`self.IsEgg`)
            (`/Engine/EditorBlueprintResources/StandardMacros.FlipFlop`
              (:`A`
                (`PaperSpriteComponent.SetSprite` (`self.NPC`) (`self.Idle1_Left`)))
              (:`B`
                (`PaperSpriteComponent.SetSprite` (`self.NPC`) (`self.Idle2_Left`))))))
        (:`then_1`
          (`KismetSystemLibrary.Delay` 10.0)
          (`/Engine/EditorBlueprintResources/StandardMacros.DoOnce` false
            (:`Completed`
              (`GameplayStatics.PlaySound2D` "/Game/Alarms/Cues/VPETAlarms_Loop_49_Cue.VPETAlarms_Loop_49_Cue" 1.0 1.0 0.0 null null)
              (`SceneComponent.SetVisibility` (`self.SoundEventSprite`) true false)
              (`KismetSystemLibrary.Delay` 5.0)
              (if (`KismetMathLibrary.RandomBool`)
                (if (`KismetMathLibrary.RandomBool`)
                  (bind _playerreference (`self.PlayerReference`)
                    (:`then`
                      (`/Game/FirstPersonBP/Blueprints/FirstPersonCharacter.SetBabySlime1` _playerreference)
                      (set `/Game/FirstPersonBP/Blueprints/FirstPersonCharacter.IsEgg` false _playerreference)
                      (set `/Game/FirstPersonBP/Blueprints/FirstPersonCharacter.IsBabySlime1` true _playerreference)
                      (set `/Game/FirstPersonBP/Blueprints/FirstPersonCharacter.IsBabySlime2` false _playerreference)
                      (set `/Game/FirstPersonBP/Blueprints/FirstPersonCharacter.IsBabySlime3` false _playerreference)
                      (set `/Game/FirstPersonBP/Blueprints/FirstPersonCharacter.IsBabySlime4` false _playerreference)
                      (set `/Game/FirstPersonBP/Blueprints/FirstPersonCharacter.IsBabySlime5` false _playerreference)
                      (`self.K2_DestroyActor` self))
                    (:`else`))
                  (else
                    (bind _playerreference_2 (`self.PlayerReference`)
                      (:`then`
                        (`/Game/FirstPersonBP/Blueprints/FirstPersonCharacter.SetBabySlime3` _playerreference_2)
                        (set `/Game/FirstPersonBP/Blueprints/FirstPersonCharacter.IsEgg` false _playerreference_2)
                        (set `/Game/FirstPersonBP/Blueprints/FirstPersonCharacter.IsBabySlime1` false _playerreference_2)
                        (set `/Game/FirstPersonBP/Blueprints/FirstPersonCharacter.IsBabySlime2` false _playerreference_2)
                        (set `/Game/FirstPersonBP/Blueprints/FirstPersonCharacter.IsBabySlime3` true _playerreference_2)
                        (set `/Game/FirstPersonBP/Blueprints/FirstPersonCharacter.IsBabySlime4` false _playerreference_2)
                        (set `/Game/FirstPersonBP/Blueprints/FirstPersonCharacter.IsBabySlime5` false _playerreference_2)
                        (`self.K2_DestroyActor` self))
                      (:`else`))))
                (elif (`KismetMathLibrary.RandomBool`)
                  (bind _playerreference_3 (`self.PlayerReference`)
                    (:`then`
                      (`/Game/FirstPersonBP/Blueprints/FirstPersonCharacter.SetBabySlime4` _playerreference_3)
                      (set `/Game/FirstPersonBP/Blueprints/FirstPersonCharacter.IsEgg` false _playerreference_3)
                      (set `/Game/FirstPersonBP/Blueprints/FirstPersonCharacter.IsBabySlime1` false _playerreference_3)
                      (set `/Game/FirstPersonBP/Blueprints/FirstPersonCharacter.IsBabySlime2` false _playerreference_3)
                      (set `/Game/FirstPersonBP/Blueprints/FirstPersonCharacter.IsBabySlime3` false _playerreference_3)
                      (set `/Game/FirstPersonBP/Blueprints/FirstPersonCharacter.IsBabySlime4` true _playerreference_3)
                      (set `/Game/FirstPersonBP/Blueprints/FirstPersonCharacter.IsBabySlime5` false _playerreference_3)
                      (`self.K2_DestroyActor` self))
                    (:`else`))
                  (elif (`KismetMathLibrary.RandomBool`)
                    (bind _playerreference_4 (`self.PlayerReference`)
                      (:`then`
                        (`/Game/FirstPersonBP/Blueprints/FirstPersonCharacter.SetBabySlime2` _playerreference_4)
                        (set `/Game/FirstPersonBP/Blueprints/FirstPersonCharacter.IsEgg` false _playerreference_4)
                        (set `/Game/FirstPersonBP/Blueprints/FirstPersonCharacter.IsBabySlime1` false _playerreference_4)
                        (set `/Game/FirstPersonBP/Blueprints/FirstPersonCharacter.IsBabySlime2` true _playerreference_4)
                        (set `/Game/FirstPersonBP/Blueprints/FirstPersonCharacter.IsBabySlime3` false _playerreference_4)
                        (set `/Game/FirstPersonBP/Blueprints/FirstPersonCharacter.IsBabySlime4` false _playerreference_4)
                        (set `/Game/FirstPersonBP/Blueprints/FirstPersonCharacter.IsBabySlime5` false _playerreference_4)
                        (`self.K2_DestroyActor` self))
                      (:`else`))
                    (else
                      (bind _playerreference_5 (`self.PlayerReference`)
                        (:`then`
                          (`/Game/FirstPersonBP/Blueprints/FirstPersonCharacter.SetBabySlime5` _playerreference_5)
                          (set `/Game/FirstPersonBP/Blueprints/FirstPersonCharacter.IsEgg` false _playerreference_5)
                          (set `/Game/FirstPersonBP/Blueprints/FirstPersonCharacter.IsBabySlime1` false _playerreference_5)
                          (set `/Game/FirstPersonBP/Blueprints/FirstPersonCharacter.IsBabySlime2` false _playerreference_5)
                          (set `/Game/FirstPersonBP/Blueprints/FirstPersonCharacter.IsBabySlime3` false _playerreference_5)
                          (set `/Game/FirstPersonBP/Blueprints/FirstPersonCharacter.IsBabySlime4` false _playerreference_5)
                          (set `/Game/FirstPersonBP/Blueprints/FirstPersonCharacter.IsBabySlime5` true _playerreference_5)
                          (`self.K2_DestroyActor` self))
                        (:`else`))))))))))
      (else
        ;[1 1 1] Rotation - Free Roam - Poop Call
        (`self.2WayRot`)
        (if (not (`self.IsInBattle`))
          (`self.PoopCleanCall`)
          (`self.FreeRoam`)
          (`self.SetEatingSprite`))))))

(event `TrainingEvent`
  (bind _charactermovement (`self.CharacterMovement`))
  (if (not (`self.IsEating`))
    (bind _outactors (`GameplayStatics.GetAllActorsOfClass` "/Game/Main/BP/TrainingPunchingBag_BP.TrainingPunchingBag_BP_C"))
    (if (not (> (`/Game/Main/BP/TrainingPunchingBag_BP.HitCount` (`|GetArrayItem` _outactors)) 4))
      (`/Engine/EditorBlueprintResources/StandardMacros.DoOnce` false :!label _label_6
        (:`Completed`
          (set `self.IsTraining` true)
          (bind _outactors_2 (`GameplayStatics.GetAllActorsOfClass` "/Game/Main/BP/VPETAttackTrainingPos.VPETAttackTrainingPos_C"))
          (`self.K2_SetActorLocation` self (`self.K2_GetActorLocation` (`|GetArrayItem` _outactors_2)) false false)
          (`CharacterMovementComponent.DisableMovement` _charactermovement)
          (`MovementComponent.StopMovementImmediately` _charactermovement)
          (set `CharacterMovementComponent.MaxWalkSpeed` 0.0 _charactermovement)
          (`KismetSystemLibrary.Delay` 1.0)
          (`GameplayStatics.PlaySound2D` "/Game/Alarms/Cues/Alarms_Loop_102_Cue1.Alarms_Loop_102_Cue1" 1.0 1.0 0.0 null null)
          (`PaperSpriteComponent.SetSprite` (`self.NPC`) (`self.Attack`))
          (bind _outactors_3 (`GameplayStatics.GetAllActorsOfClass` "/Game/Main/BP/VPETAttackTrainingPos.VPETAttackTrainingPos_C"))
          (bind (_returnvalue_roll _returnvalue_pitch _returnvalue_yaw) (`KismetMathLibrary.BreakRotator` (`self.K2_GetActorRotation` (`|GetArrayItem` _outactors_3))))
          (`|SpawnActorFromClass` (`self.AttackParticleClass`) (`KismetMathLibrary.MakeTransform` (`SceneComponent.K2_GetComponentLocation` (`self.AttackPoint`)) (`KismetMathLibrary.MakeRotator` 0.0 0.0 (- _returnvalue_yaw 90.0))) "AlwaysSpawn" "OverrideRootScale" null null)
          (`KismetSystemLibrary.Delay` 1.0)
          (`PaperSpriteComponent.SetSprite` (`self.NPC`) (`self.Idle1_Left`))
          (bind _outactors_4 (`GameplayStatics.GetAllActorsOfClass` "/Game/Main/BP/TrainingPunchingBag_BP.TrainingPunchingBag_BP_C"))
          (`/Game/Main/BP/TrainingPunchingBag_BP.ResetCanTrainNeomon` (`|GetArrayItem` _outactors_4)))))))

(event `ResetTrainingEvent`
  (goto _label_6 :!via `Reset`))

(event `SetEatingSprite`
  (bind _npc (`self.NPC`))
  (if (and (`self.IsFreeRoaming`) (`self.IsInBattle`) (`self.IsTraining`) (`self.IsEgg`))
    _
    (elif (`self.IsEating`)
      (`KismetSystemLibrary.Delay` 1.0)
      (`/Engine/EditorBlueprintResources/StandardMacros.FlipFlop`
        (:`A`
          (`PaperSpriteComponent.SetSprite` _npc (`self.Idle1_Left`)))
        (:`B`
          (`PaperSpriteComponent.SetSprite` _npc (`self.Eat`)))))))

(event `SetVpetWalk`
  (bind _charactermovement (`self.CharacterMovement`))
  (`CharacterMovementComponent.SetMovementMode` _charactermovement "MOVE_Walking" 0)
  (set `CharacterMovementComponent.MaxWalkSpeed` 100.0 _charactermovement))

(event `FreeRoam`
  (bind _charactermovement (`self.CharacterMovement`))
  (if (`self.IsTraining`)
    (`MovementComponent.StopMovementImmediately` _charactermovement)
    (set `CharacterMovementComponent.MaxWalkSpeed` 0.0 _charactermovement)
    (else
      (if (not (`self.IsFreeRoaming`)) :!label _label_7
        (`KismetSystemLibrary.Delay` (`KismetMathLibrary.RandomFloatInRange` 1.0 3.0))
        (if (`KismetMathLibrary.RandomBool`)
          (if (`KismetMathLibrary.RandomBool`)
            (set `self.IsFreeRoaming` true)
            (bind _outactors (`GameplayStatics.GetAllActorsOfClass` "/Game/Main/BP/VPETLeftPos.VPETLeftPos_C"))
            (`|AIMoveTo` self (0.0 0.0 0.0) (`|GetArrayItem` _outactors) 1.0
              (:`OnSuccess`
                _)
              (:`OnFail`
                _))
            (set `self.IsFreeRoaming` false)
            (`KismetSystemLibrary.Delay` 2.0)
            (`self.ResetFreeRoam`)
            (else
              (set `self.IsFreeRoaming` true)
              (bind _outactors_2 (`GameplayStatics.GetAllActorsOfClass` "/Game/Main/BP/VPETMiddlePos.VPETMiddlePos_C"))
              (`|AIMoveTo` self (0.0 0.0 0.0) (`|GetArrayItem` _outactors_2) 1.0
                (:`OnSuccess`
                  _)
                (:`OnFail`
                  _))
              (set `self.IsFreeRoaming` false)
              (`KismetSystemLibrary.Delay` 2.0)
              (`self.ResetFreeRoam`)))
          (elif (`KismetMathLibrary.RandomBool`)
            (set `self.IsFreeRoaming` true)
            (bind _outactors_3 (`GameplayStatics.GetAllActorsOfClass` "/Game/Main/BP/VPETRightPos.VPETRightPos_C"))
            (`|AIMoveTo` self (0.0 0.0 0.0) (`|GetArrayItem` _outactors_3) 1.0
              (:`OnSuccess`
                _)
              (:`OnFail`
                _))
            (set `self.IsFreeRoaming` false)
            (`KismetSystemLibrary.Delay` 2.0)
            (`self.ResetFreeRoam`)
            (else
              (set `self.IsFreeRoaming` true)
              (bind _outactors_4 (`GameplayStatics.GetAllActorsOfClass` "/Game/Main/BP/VPETFrontMiddlePos.VPETFrontMiddlePos_C"))
              (`|AIMoveTo` self (0.0 0.0 0.0) (`|GetArrayItem` _outactors_4) 1.0
                (:`OnSuccess`
                  _)
                (:`OnFail`
                  _))
              (set `self.IsFreeRoaming` false)
              (`KismetSystemLibrary.Delay` 2.0)
              (`self.ResetFreeRoam`))))))))

(event `ResetFreeRoam`
  (`/Engine/EditorBlueprintResources/StandardMacros.DoOnce` false :!via `Reset`
    (:`Completed`
      (goto _label_7))))

(event `TimerPooEvent`
  (params (Duration :type "Float (double-precision)"))
  (`KismetSystemLibrary.Delay` Duration)
  (`|SpawnActorFromClass` "/Game/Main/BP/NeoPoo_BP.NeoPoo_BP_C" (`KismetMathLibrary.MakeTransform` (`SceneComponent.K2_GetComponentLocation` (`self.PoopPosition`))) "AlwaysSpawn" "OverrideRootScale" null null :!label _label_8)
  (bind _playerreference (`self.PlayerReference`)
    (:`then`
      (set `self.NeedsCleaning` true)
      (set `/Game/FirstPersonBP/Blueprints/FirstPersonCharacter.NeedCleaning` true _playerreference))
    (:`else`)))

(event `PooEvent`
  (`KismetSystemLibrary.Delay` (`KismetMathLibrary.RandomFloatInRange` 150.0 400.0))
  (goto _label_8))

(event `PoopCleanCall`
  (if (`self.NeedsCleaning`)
    (`/Engine/EditorBlueprintResources/StandardMacros.DoOnce` false :!label _label_9
      (:`Completed`
        (`SceneComponent.SetVisibility` (`self.PoopEventSprite`) true false)
        (`GameplayStatics.PlaySound2D` "/Game/Alarms/Cues/Alarms_Loop_91_Cue.Alarms_Loop_91_Cue" 1.0 1.0 0.0 null null)
        (`KismetSystemLibrary.Delay` 10.0)
        (`SceneComponent.SetVisibility` (`self.PoopEventSprite`) false false)
        (`KismetSystemLibrary.Delay` 20.0)
        (goto _label_9 :!via `Reset`)))))

(event `ResetRot`
  (goto _label_10 :!via `Reset`))

(event `2WayRot`
  (bind _returnvalue (`KismetMathLibrary.Normal` (- (`self.K2_GetActorLocation` (`GameplayStatics.GetPlayerCharacter` 0)) (`self.K2_GetActorLocation` self))))
  (set `self.Degrees` (`KismetMathLibrary.DegAcos` (`KismetMathLibrary.Dot_VectorVector` (`self.GetActorForwardVector`) _returnvalue)))
  (`/Engine/EditorBlueprintResources/StandardMacros.DoOnce` false :!label _label_10
    (:`Completed`
      (if (or (`self.IsEating`) (`self.IsTraining`) (`self.IsInBattle`))
        (`self.ResetRot`)
        (elif (< (`KismetMathLibrary.Dot_VectorVector` (`self.GetActorRightVector`) _returnvalue) 0.0)
          (`/Engine/EditorBlueprintResources/StandardMacros.CompareFloat` (`self.Degrees`) 90.0
            (:`>`
              _)
            (:`==`
              _)
            (:`<`
              _))
          (if (> (`KismetMathLibrary.VSize` (`self.GetVelocity`)) 0.01)
            ;[1 1 1] Left Walk
            (`PaperSpriteComponent.SetSprite` (`self.NPC`) (`self.LLegWalkLeft`))
            (`KismetSystemLibrary.Delay` (`self.WalkSpritesFrameAnimDelay`))
            (`PaperSpriteComponent.SetSprite` (`self.NPC`) (`self.RLegWalkLeft`))
            (`KismetSystemLibrary.Delay` (`self.WalkSpritesFrameAnimDelay`))
            (`self.ResetRot`)
            (else
              ;[1 1 1] Left Idle
              (`PaperSpriteComponent.SetSprite` (`self.NPC`) (`self.Idle1_Left`))
              (`KismetSystemLibrary.Delay` (`self.IdleSpritesFrameAnimDelay`))
              (`PaperSpriteComponent.SetSprite` (`self.NPC`) (`self.Idle2_Left`))
              (`KismetSystemLibrary.Delay` (`self.IdleSpritesFrameAnimDelay`))
              (`self.ResetRot`)))
          (else
            (`/Engine/EditorBlueprintResources/StandardMacros.CompareFloat` (`self.Degrees`) 45.0
              (:`>`
                _)
              (:`==`
                _)
              (:`<`
                _))
            (if (> (`KismetMathLibrary.VSize` (`self.GetVelocity`)) 0.01)
              ;[1 1 1] Right Walk
              (`PaperSpriteComponent.SetSprite` (`self.NPC`) (`self.LLegWalk_Right`))
              (`KismetSystemLibrary.Delay` (`self.WalkSpritesFrameAnimDelay`))
              (`PaperSpriteComponent.SetSprite` (`self.NPC`) (`self.RLegWalk_Right`))
              (`KismetSystemLibrary.Delay` (`self.WalkSpritesFrameAnimDelay`))
              (`self.ResetRot`)
              (else
                ;[1 1 1] Right Idle
                (`PaperSpriteComponent.SetSprite` (`self.NPC`) (`self.Idle1_Right`))
                (`KismetSystemLibrary.Delay` (`self.IdleSpritesFrameAnimDelay`))
                (`PaperSpriteComponent.SetSprite` (`self.NPC`) (`self.Idle2_Right`))
                (`KismetSystemLibrary.Delay` (`self.IdleSpritesFrameAnimDelay`))
                (`self.ResetRot`)))))))))

(fn `FacePlayerCamera`
  (bind _npc (`self.NPC`))
  (bind _eventlowstrengthsprite (`self.EventLowStrengthSprite`))
  (bind _poopeventsprite (`self.PoopEventSprite`))
  (bind _eventhungersprite (`self.EventHungerSprite`))
  (bind _soundeventsprite (`self.SoundEventSprite`))
  (bind (_returnvalue_roll _returnvalue_pitch _returnvalue_yaw) (`KismetMathLibrary.BreakRotator` (`KismetMathLibrary.FindLookAtRotation` (`SceneComponent.K2_GetComponentLocation` _poopeventsprite) (`SceneComponent.K2_GetComponentLocation` (`/Game/FirstPersonBP/Blueprints/FirstPersonCharacter.FirstPersonCamera` (`self.PlayerReference`))))))
  (bind (_returnvalue_roll_2 _returnvalue_pitch_2 _returnvalue_yaw_2) (`KismetMathLibrary.BreakRotator` (`KismetMathLibrary.FindLookAtRotation` (`SceneComponent.K2_GetComponentLocation` _eventhungersprite) (`SceneComponent.K2_GetComponentLocation` (`/Game/FirstPersonBP/Blueprints/FirstPersonCharacter.FirstPersonCamera` (`self.PlayerReference`))))))
  (bind (_returnvalue_roll_3 _returnvalue_pitch_3 _returnvalue_yaw_3) (`KismetMathLibrary.BreakRotator` (`KismetMathLibrary.FindLookAtRotation` (`SceneComponent.K2_GetComponentLocation` _soundeventsprite) (`SceneComponent.K2_GetComponentLocation` (`/Game/FirstPersonBP/Blueprints/FirstPersonCharacter.FirstPersonCamera` (`self.PlayerReference`))))))
  (bind (_returnvalue_roll_4 _returnvalue_pitch_4 _returnvalue_yaw_4) (`KismetMathLibrary.BreakRotator` (`KismetMathLibrary.FindLookAtRotation` (`SceneComponent.K2_GetComponentLocation` _eventlowstrengthsprite) (`SceneComponent.K2_GetComponentLocation` (`/Game/FirstPersonBP/Blueprints/FirstPersonCharacter.FirstPersonCamera` (`self.PlayerReference`))))))
  (bind (_returnvalue_roll_5 _returnvalue_pitch_5 _returnvalue_yaw_5) (`KismetMathLibrary.BreakRotator` (`KismetMathLibrary.FindLookAtRotation` (`SceneComponent.K2_GetComponentLocation` _npc) (`SceneComponent.K2_GetComponentLocation` (`/Game/FirstPersonBP/Blueprints/FirstPersonCharacter.FirstPersonCamera` (`self.PlayerReference`))))))
  (`SceneComponent.K2_SetWorldRotation` _npc (`KismetMathLibrary.MakeRotator` 0.0 0.0 (- _returnvalue_yaw_5 90.0)) false false)
  (`SceneComponent.K2_SetWorldRotation` _eventhungersprite (`KismetMathLibrary.MakeRotator` 0.0 0.0 (- _returnvalue_yaw_2 90.0)) false false)
  (`SceneComponent.K2_SetWorldRotation` _soundeventsprite (`KismetMathLibrary.MakeRotator` 0.0 0.0 (- _returnvalue_yaw_3 90.0)) false false)
  (`SceneComponent.K2_SetWorldRotation` _eventlowstrengthsprite (`KismetMathLibrary.MakeRotator` 0.0 0.0 (- _returnvalue_yaw_4 90.0)) false false)
  (`SceneComponent.K2_SetWorldRotation` _poopeventsprite (`KismetMathLibrary.MakeRotator` 0.0 0.0 (- _returnvalue_yaw 90.0)) false false)
  (return))

(fn `UserConstructionScript`)