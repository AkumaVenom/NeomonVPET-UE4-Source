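; Cleaner_BP is an actor whose Cleaner component continually turns to face the player.
; BeginPlay casts player character 0 to FirstPersonCharacter and caches the reference.
; Every Tick, FacePlayer computes a look-at rotation from Cleaner to the player's first-person camera.
; It applies only the yaw, offset by a quarter turn, keeping pitch and roll at zero so Cleaner stays upright.
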(event `self.ReceiveBeginPlay`
  (bind _asfirst_person_character (cast `/Game/FirstPersonBP/Blueprints/FirstPersonCharacter` (`GameplayStatics.GetPlayerCharacter` 0)))
  (set `self.PlayerReference` _asfirst_person_character))

(event `self.ReceiveTick`
  (params (DeltaSeconds :type "Float (single-precision)"))
  (`self.FacePlayer`))

(fn `FacePlayer`
  (bind _cleaner (`self.Cleaner`))
  (bind (_returnvalue_roll _returnvalue_pitch _returnvalue_yaw) (`KismetMathLibrary.BreakRotator` (`KismetMathLibrary.FindLookAtRotation` (`SceneComponent.K2_GetComponentLocation` _cleaner) (`SceneComponent.K2_GetComponentLocation` (`/Game/FirstPersonBP/Blueprints/FirstPersonCharacter.FirstPersonCamera` (`self.PlayerReference`))))))
  (`SceneComponent.K2_SetWorldRotation` _cleaner (`KismetMathLibrary.MakeRotator` 0.0 0.0 (- _returnvalue_yaw 90.0)) false false)
  (return))

(fn `UserConstructionScript`)